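; Player controller Blueprint that sets up the main player HUD when play begins.
; On BeginPlay it caches player pawn 0 as a bp-PlayerCharacter reference, then creates the WPlayerMain widget and adds it to the viewport.
; It then passes that character to the HP bar and posture bar sub-widgets through their init events.
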(event `self.ReceiveBeginPlay`
  (`|ExecutionSequence`
    (:`then_0`
      (bind _asbp__player_character (cast `/Game/Blueprints/Character/Player/bp-PlayerCharacter` (`GameplayStatics.GetPlayerPawn` 0)))
      (set `self.PlayerRef` _asbp__player_character))
    (:`then_1`
      (bind _returnvalue (`|CreateWidget` "/Game/UI/w-PlayerMain.w-PlayerMain_C"))
      (bind _output_get (set `self.mainWidget` _returnvalue))
      (`UserWidget.AddToViewport` _output_get 0))
    (:`then_2`
      (`/Game/UI/w-PlayerHpBar.e-PlayerHpInit` (`/Game/UI/w-PlayerMain.w-PlayerHpBar` (`self.mainWidget`)) (`self.PlayerRef`)))
    (:`then_3`
      (`/Game/UI/w-PlayerPostureBar.e-PlayerPostureInit` (`/Game/UI/w-PlayerMain.w-PlayerPostureBar` (`self.mainWidget`)) (`self.PlayerRef`)))))

(fn `UserConstructionScript`)
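; Bonfire actor that offers itself as an interactable to the player character when nearby.
; Its Sphere overlap events register and unregister the bonfire with the player's C_InteractionComponent, ignoring actors that are not bp-PlayerCharacter.
; The Widget component is hidden on BeginPlay, and this graph contains no logic to show it or respond to an interaction.
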(event `self.ReceiveBeginPlay`
  (`SceneComponent.SetVisibility` (`self.Widget`) false false))

(event `self.Sphere.OnComponentBeginOverlap`
  (params (OverlappedComponent :type "PrimitiveComponent Object Reference") (OtherActor :type "Actor Object Reference") (OtherComp :type "PrimitiveComponent Object Reference") (OtherBodyIndex :type Integer) (bFromSweep :type Boolean) (SweepResult :type "HitResult Structure (by ref)"))
  (bind _asbp__player_character (cast `/Game/Blueprints/Character/Player/bp-PlayerCharacter` OtherActor))
  (`C_InteractionComponent.registerInteractable` (`self.GetComponentByClass` _asbp__player_character "/Script/ProjectARPG.C_InteractionComponent") self))

(event `self.Sphere.OnComponentEndOverlap`
  (params (OverlappedComponent :type "PrimitiveComponent Object Reference") (OtherActor :type "Actor Object Reference") (OtherComp :type "PrimitiveComponent Object Reference") (OtherBodyIndex :type Integer))
  (bind _asbp__player_character (cast `/Game/Blueprints/Character/Player/bp-PlayerCharacter` OtherActor))
  (`C_InteractionComponent.unregisterInteractable` (`self.GetComponentByClass` _asbp__player_character "/Script/ProjectARPG.C_InteractionComponent") self))

(fn `UserConstructionScript`)